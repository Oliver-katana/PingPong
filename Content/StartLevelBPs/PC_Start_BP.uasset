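; PC_Start_BP is a player controller, apparently for the start level, that opens the main menu widget.
; On BeginPlay, if locally controlled, it creates W_Menu_BP, stores it, adds it to the viewport, shows the cursor and sets UI-only input focused on the menu.
; When destroyed, it hides the cursor and restores game-only input.
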(event `self.ReceiveBeginPlay`
  (if (`self.IsLocalController`)
    (bind _returnvalue (`|CreateWidget` "/Game/UI/W_Menu_BP.W_Menu_BP_C"))
    (bind _output_get (set `self.W_Menu_Ref` _returnvalue))
    (`UserWidget.AddToViewport` _output_get 0)
    (set `self.bShowMouseCursor` true)
    (`WidgetBlueprintLibrary.SetInputMode_UIOnlyEx` self _output_get)))

(event `self.ReceiveDestroyed`
  (set `self.bShowMouseCursor` false)
  (`WidgetBlueprintLibrary.SetInputMode_GameOnly` self))

(fn `UserConstructionScript`)