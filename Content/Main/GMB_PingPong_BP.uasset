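; Game mode for a two-player ping-pong match that seats players as they log in and starts play once both are connected.
; PostLogin stores each controller, then spawns and possesses a paddle pawn at a tagged start: Start1 for the first player, Start2 for the second.
; The second login also triggers a delayed ball spawn, then has the GameState multicast removal of the waiting widget.
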(event `self.K2_PostLogin`
  (params (NewPlayer :type "PlayerController Object Reference"))
  (bind _playercontrollersarray (`self.PlayerControllersArray`))
  (bind _output (`|GetArrayItem` _playercontrollersarray))
  (bind _output_2 (`|GetArrayItem` (`self.PlayerControllersArray`) 1))
  ;[1 1 1] Check for both players connected and save their controllers
  (bind _returnvalue (`KismetArrayLibrary.Array_Add` _playercontrollersarray NewPlayer))
  (if (== _returnvalue 1)
    (bind _outactors (`GameplayStatics.GetAllActorsWithTag` "Start2"))
    (bind _returnvalue_2 (`|SpawnActorFromClass` "/Game/Player/P_Player_BP.P_Player_BP_C" (`self.GetTransform` (`|GetArrayItem` _outactors)) "AlwaysSpawn" "SelectDefaultAtRuntime" _output_2 null))
    (`Controller.Possess` _output_2 _returnvalue_2)
    (`KismetSystemLibrary.Delay` 0.5)
    (`self.SpawnBall`)
    (`KismetSystemLibrary.Delay` 0.2)
    (bind _asgsb_ping_pong_bp (cast `/Game/Main/GSB_PingPong_BP` (`GameplayStatics.GetGameState`)))
    (`/Game/Main/GSB_PingPong_BP.RemoveWaitingWidget_Multicast` _asgsb_ping_pong_bp (`self.PlayerControllersArray`))
    (else
      (bind _outactors_2 (`GameplayStatics.GetAllActorsWithTag` "Start1"))
      (bind _returnvalue_3 (`|SpawnActorFromClass` "/Game/Player/P_Player_BP.P_Player_BP_C" (`self.GetTransform` (`|GetArrayItem` _outactors_2)) "AlwaysSpawn" "SelectDefaultAtRuntime" _output null))
      (`Controller.Possess` _output _returnvalue_3))))

(fn `UserConstructionScript`)